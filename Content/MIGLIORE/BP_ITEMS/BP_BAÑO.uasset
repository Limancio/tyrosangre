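; Bathroom door actor that swings open away from or toward a side based on the player's position, and shuts again when triggered while open.
; Overlap with the third-person character toggles CanDoAction, while Tick consumes an OnAction flag that this graph never sets itself.
; A dot product picks the swing direction, then Tick steps yaw from the original rotation, snapping near closed and playing movement sounds.
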(event `self.ReceiveBeginPlay`
  (set `self.player_reference` (`GameplayStatics.GetPlayerCharacter` 0))
  (set `self.origin_rotator` (`self.K2_GetActorRotation`)))

(event `self.ReceiveActorBeginOverlap`
  (params (OtherActor :type "Actor Object Reference"))
  (if (`GameplayStatics.ObjectIsA` OtherActor "/Game/ThirdPerson/Blueprints/BP_ThirdPersonCharacter.BP_ThirdPersonCharacter_C")
    (set `self.can_do_action` true)))

(event `self.ReceiveActorEndOverlap`
  (params (OtherActor :type "Actor Object Reference"))
  (if (`GameplayStatics.ObjectIsA` OtherActor "/Game/ThirdPerson/Blueprints/BP_ThirdPersonCharacter.BP_ThirdPersonCharacter_C")
    (set `self.can_do_action` false)))

(event `self.ReceiveTick`
  (params (DeltaSeconds :type "Float (single-precision)"))
  (set `self.dt_per_frame` DeltaSeconds)
  (if (`self.on_action`)
    ;[1 1 1] check direction
    (set `self.on_action` false)
    (`GameplayStatics.PlaySoundAtLocation` "/Game/MIGLIORE/BP_ITEMS/door_closing.door_closing" (`self.K2_GetActorLocation`) (struct) 1.0 1.0 0.0 null null null null)
    (if (!= (`self.current_direction`) 0.0)
      (set `self.target_direction` 0.0)
      (elif (> (`KismetMathLibrary.RadiansToDegrees` (`KismetMathLibrary.Dot_VectorVector` (`KismetMathLibrary.GetRightVector` (`self.origin_rotator`)) (`KismetMathLibrary.Normal` (- (`KismetMathLibrary.MakeVector` (.x (`self.K2_GetActorLocation`)) (.y (`self.K2_GetActorLocation`))) (`KismetMathLibrary.MakeVector` (.x (`self.K2_GetActorLocation` (`self.player_reference`))) (.y (`self.K2_GetActorLocation` (`self.player_reference`)))))))) 0.0)
        (set `self.target_direction` 90.0)
        (else
          (set `self.target_direction` -90.0))))
    (else
      ;[1 1 1] mover
      (if (!= (`self.current_direction`) (`self.target_direction`))
        (if (>= (`self.current_direction`) (`self.target_direction`))
          (set `self.current_direction` (`KismetMathLibrary.FClamp` (- (`self.current_direction`) (* (`self.dt_per_frame`) (`self.blend_factor`))) -90.0 90.0))
          (else
            (set `self.current_direction` (`KismetMathLibrary.FClamp` (+ (`self.current_direction`) (* (`self.dt_per_frame`) (`self.blend_factor`))) -90.0 90.0))))
        (if (== (`self.target_direction`) 0.0)
          (if (and (<= (`self.current_direction`) 10.0) (>= (`self.current_direction`) -10.0))
            (set `self.current_direction` 0.0)))
        (`self.K2_SetActorRotation` (`KismetMathLibrary.ComposeRotators` (`self.origin_rotator`) (`KismetMathLibrary.MakeRotator` 0.0 0.0 (`self.current_direction`))))
        (if (== (`self.current_direction`) (`self.target_direction`))
          (`GameplayStatics.PlaySoundAtLocation` "/Game/MIGLIORE/BP_ITEMS/door_close.door_close" (`self.K2_GetActorLocation`) (struct) 1.0 1.0 0.0 null null null null))))))

(fn `UserConstructionScript`)