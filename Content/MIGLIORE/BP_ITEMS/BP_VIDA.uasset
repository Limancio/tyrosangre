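; BP_VIDA is a health pickup that heals the player when touched.
; On BeginPlay it caches the third-person character reference.
; When that character overlaps it, it adds health clamped to the maximum, refreshes the character's material through UpdateMiglioMaterial, destroys itself and plays a 2D heal sound.
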(event `self.ReceiveBeginPlay`
  (bind _returnvalue (`GameplayStatics.GetActorOfClass` "/Game/ThirdPerson/Blueprints/BP_ThirdPersonCharacter.BP_ThirdPersonCharacter_C"))
  (set `self.player_reference` _returnvalue))

(event `self.ReceiveActorBeginOverlap`
  (params (OtherActor :type "Actor Object Reference"))
  (if (`GameplayStatics.ObjectIsA` OtherActor "/Game/ThirdPerson/Blueprints/BP_ThirdPersonCharacter.BP_ThirdPersonCharacter_C")
    (set `/Game/ThirdPerson/Blueprints/BP_ThirdPersonCharacter.game_curr_health` (`KismetMathLibrary.FClamp` (+ (`/Game/ThirdPerson/Blueprints/BP_ThirdPersonCharacter.game_curr_health` (`self.player_reference`)) 50.0) 0.0 100.0) (`self.player_reference`))
    (`/Game/ThirdPerson/Blueprints/BP_ThirdPersonCharacter.update_miglio_material` (`self.player_reference`))
    (`self.K2_DestroyActor`)
    (`GameplayStatics.PlaySound2D` "/Game/MIGLIORE/BP_ITEMS/pick_heal.pick_heal" 1.0 1.0 0.0 null null)))

(fn `UserConstructionScript`)